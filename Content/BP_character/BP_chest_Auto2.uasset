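; BP_chest_Auto2 is a chest Blueprint that can be opened once through an Interact event.
; On first interaction it sets Opened, increments its CoinsToGive, rolls the Scene component by 30 degrees and prints a debug message.
; CanInteract reports true only while the chest is closed; Interact checks Opened directly.
; The coin count is not passed to any other object, and the logic that resets Opened is unconnected.
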(event EventBeginPlay)

(event Collision|EventActorBeginOverlap
  (params (OtherActor :type Actor%20Object%20Reference)))

(event EventTick
  (params (DeltaSeconds :type Float%20%28single-precision%29)))

(event EventInteract
  (bind _scene (Variables|Default|GetScene))
  (bind _returnvalue (Transformation|GetRelativeTransform _scene))
  (if (not (Variables|Default|GetbOpened))
    (Variables|Default|SetCoinsToGive (+ (Variables|Default|GetCoinsToGive) 1))
    (Variables|Default|SetbOpened true)
    (Transformation|SetRelativeTransform _scene (Math|Transform|MakeTransform "0, 0, 0" (Math|Rotator|MakeRotator (+ (.roll (.rotation _returnvalue)) 3e+01) (.pitch (.rotation _returnvalue)) (.yaw (.rotation _returnvalue))) "1.000000,1.000000,1.000000") false false)
    (Development|PrintString "coins++")))

(fn ConstructionScript)

(fn CanInteract
  (if (Variables|Default|GetbOpened)
    (return false)
    (else
      (return true))))