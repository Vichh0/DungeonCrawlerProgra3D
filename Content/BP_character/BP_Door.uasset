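; BP_Door is an interactable door actor that opens once and cannot be closed again.
; On Interact, if not already open, it sets the Open flag, instantly adds a quarter turn of yaw to the Scene component's relative rotation, and prints a debug message.
; CanInteract returns false once the door is open, so further interaction is refused.
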(event EventBeginPlay)

(event Collision|EventActorBeginOverlap
  (params (OtherActor :type Actor%20Object%20Reference)))

(event EventTick
  (params (DeltaSeconds :type Float%20%28single-precision%29)))

(event EventInteract
  (bind _scene (Variables|Default|GetScene))
  (bind _returnvalue (Transformation|GetRelativeTransform _scene))
  (if (not (Variables|Default|GetOpen))
    (Variables|Default|SetOpen true)
    (Transformation|SetRelativeTransform _scene (Math|Transform|MakeTransform (.location _returnvalue) (Math|Rotator|MakeRotator (.roll (.rotation _returnvalue)) (.pitch (.rotation _returnvalue)) (+ (.yaw (.rotation _returnvalue)) 9e+01)) (.scale _returnvalue)) false false)
    (Development|PrintString "Door Opened")))

(fn ConstructionScript)

(fn CanInteract
  (if (Variables|Default|GetOpen)
    (return false)
    (else
      (return true))))